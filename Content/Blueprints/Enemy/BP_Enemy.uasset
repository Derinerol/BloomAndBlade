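; Enemy character that melees the player, takes damage and drops a flower pickup on death.
; The swing attack plays a montage, then damages player characters found by a delayed sphere overlap ahead, with a cooldown.
; TakeDamage reveals and updates a health widget, launches along the player's forward vector, then stops movement, with effects and sound.
; A self-rescheduling loop plays attached ambient sound at random intervals until death, which disables collision and movement.
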(event OnComponentBeginOverlap(CapsuleComponent)
  (params (OverlappedComponent :type Primitive%20Component%20Object%20Reference) (OtherActor :type Actor%20Object%20Reference) (OtherComp :type Primitive%20Component%20Object%20Reference) (OtherBodyIndex :type Integer) (bFromSweep :type Boolean) (SweepResult :type Hit%20Result%20Structure%20%28by%20ref%29))
  (if (Actor|ActorHasTag OtherActor "Player")
    (Utilities|Casting|CastToBP_ThirdPersonCharacter OtherActor)))

(event Custom|ExecuteSwingAttack
  (if (not (Variables|Default|GetIsDead))
    (if (Variables|Default|GetCanAttack)
      (Variables|Default|SetCanAttack false)
      (Animation|Montage|PlayMontage (Variables|Character|GetMesh) (Variables|Default|GetAttackMontage)
        (:then
          (Utilities|FlowControl|Delay 1.0)
          (bind _outactors (Collision|SphereOverlapActors (+ (Transformation|GetActorLocation) (* (Transformation|GetActorForwardVector) 1e+02)) 8e+01 (Utilities|Array|MakeArray "ObjectTypeQuery3") 0))
          (for _array_element _outactors
            (bind _asbp_third_person_character (Utilities|Casting|CastToBP_ThirdPersonCharacter _array_element))
            (Default|TakeDamage _asbp_third_person_character (Variables|Default|GetDamage)))
          (Utilities|FlowControl|Delay 1.5)
          (Variables|Default|SetCanAttack true))))))

(event Custom|Event_Die
  (Variables|Default|SetIsDead true)
  (Animation|Montage|PlayMontage (Variables|Character|GetMesh) (Variables|Default|GetDeathMontage)
    (:then
      (Collision|SetCollisionEnabled (Variables|Collision|GetCapsuleComponent) "NoCollision")
      (Pawn|Components|CharacterMovement|DisableMovement (Variables|Character|GetCharacterMovement))
      (Components|DestroyComponent (Variables|Default|GetEnemyHealthWidget))
      (Utilities|FlowControl|Delay 2.2)
      (Game|SpawnActorfromClass "/Game/Blueprints/Flower/BP_FlowerPickup.BP_FlowerPickup_C" (Math|Conversions|ToTransform(Vector) (- (Transformation|GetActorLocation) "0.000000,0.000000,95.000000")) "Undefined" "MultiplyWithRoot" 0 "NewEnumerator0" 0))))

(event Custom|Loop_PlayAmbientSound
  (if (not (Variables|Default|GetIsDead))
    (Audio|SpawnSoundAttached "/Game/AudioFiles/Enemy/SC_EnemyAmbient.SC_EnemyAmbient" (Variables|Character|GetMesh) "None" "0, 0, 0" "0, 0, 0" "KeepRelativeOffset" false 1.0 1.0 0.0 "/Game/AudioSettings/SA_EnemyProximity.SA_EnemyProximity" 0)
    (Utilities|FlowControl|Delay (Math|Random|RandomFloatinRange 8.0 2e+01))
    (CallFunction|LoopPlayAmbientSound)))

(event EventBeginPlay
  (CallFunction|LoopPlayAmbientSound)
  (bind _aswbp_enemy_health (Utilities|Casting|CastToWBP_EnemyHealth (UserInterface|GetUserWidgetObject (Variables|Default|GetEnemyHealthWidget))))
  (Variables|Default|SetEnemyHealthUI _aswbp_enemy_health))

(event Collision|EventActorBeginOverlap
  (params (OtherActor :type Actor%20Object%20Reference)))

(fn ConstructionScript)

(fn TakeDamage
  (params (Damage :type Float%20%28double-precision%29))
  (bind _returnvalue (Transformation|GetActorLocation))
  (if (not (Variables|Default|GetIsDead))
    (Rendering|SetVisibility (Variables|Default|GetEnemyHealthWidget) true false)
    (bind _output_get (Variables|Default|SetHealth (- (Variables|Default|GetHealth) Damage)))
    (Character|LaunchCharacter (* (Transformation|GetActorForwardVector (Game|GetPlayerCharacter 0)) 8e+02) true false)
    (Effects|SpawnEmitteratLocation 0 _returnvalue)
    (Components|Movement|StopMovementImmediately (Variables|Character|GetCharacterMovement))
    (Default|SetHealthPercent (Variables|Default|GetEnemyHealthUI) (/ (Variables|Default|GetHealth) (Variables|Default|GetMaxHealth)))
    (Audio|PlaySoundatLocation 0 _returnvalue "0, 0, 0" 1.0 1.0 0.0 0 0 0 0)
    (if (<= _output_get 0.0)
      (CallFunction|EventDie))))