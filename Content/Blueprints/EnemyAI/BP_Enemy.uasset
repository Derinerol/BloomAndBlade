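; Enemy character Blueprint with a melee swing attack, health and an overhead or on-screen health widget.
; ExecuteSwingAttack runs a sphere overlap in front of the enemy, damages player characters found, then waits out a cooldown.
; TakeDamage reduces health, launches the enemy along the player's forward vector, spawns an emitter and updates the widget.
; At zero health it spawns an actor at its location and destroys itself.
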(event OnComponentBeginOverlap(CapsuleComponent)
  (params (OverlappedComponent :type Primitive%20Component%20Object%20Reference) (OtherActor :type Actor%20Object%20Reference) (OtherComp :type Primitive%20Component%20Object%20Reference) (OtherBodyIndex :type Integer) (bFromSweep :type Boolean) (SweepResult :type Hit%20Result%20Structure%20%28by%20ref%29))
  (if (Actor|ActorHasTag OtherActor "Player")
    (Utilities|Casting|CastToBP_ThirdPersonCharacter OtherActor)))

(event Custom|ExecuteSwingAttack
  (if (Variables|Default|GetCanAttack)
    (Variables|Default|SetCanAttack false)
    (bind _outactors (Collision|SphereOverlapActors (+ (Transformation|GetActorLocation) (* (Transformation|GetActorForwardVector) 1e+02)) 8e+01 (Utilities|Array|MakeArray "ObjectTypeQuery3") 0))
    (for _array_element _outactors
      (bind _asbp_third_person_character (Utilities|Casting|CastToBP_ThirdPersonCharacter _array_element))
      (Default|TakeDamage _asbp_third_person_character (Variables|Default|GetDamage)))
    (Utilities|FlowControl|Delay 1.5)
    (Variables|Default|SetCanAttack true)))

(event EventBeginPlay
  (bind _aswbp_enemy_health (Utilities|Casting|CastToWBP_EnemyHealth (UserInterface|GetUserWidgetObject (Variables|Default|GetEnemyHealthWidget))))
  (Variables|Default|SetEnemyHealthUI _aswbp_enemy_health))

(event Collision|EventActorBeginOverlap
  (params (OtherActor :type Actor%20Object%20Reference)))

(fn ConstructionScript)

(fn TakeDamage
  (params (Damage :type Float%20%28double-precision%29))
  (bind _output_get (Variables|Default|SetHealth (- (Variables|Default|GetHealth) Damage)))
  (Character|LaunchCharacter (* (Transformation|GetActorForwardVector (Game|GetPlayerCharacter 0)) 8e+02) true false)
  (Effects|SpawnEmitteratLocation 0 (Transformation|GetActorLocation))
  (Components|Movement|StopMovementImmediately (Variables|Character|GetCharacterMovement))
  (Default|SetHealthPercent (Variables|Default|GetEnemyHealthUI) (/ (Variables|Default|GetHealth) (Variables|Default|GetMaxHealth)))
  (if (<= _output_get 0.0)
    (Game|SpawnActorfromClass "/Game/Blueprints/Flower/BP_FlowerPickup.BP_FlowerPickup_C" (Math|Conversions|ToTransform(Vector) (Transformation|GetActorLocation)) "Undefined" "MultiplyWithRoot" 0 0)
    (Actor|DestroyActor)))