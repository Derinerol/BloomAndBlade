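; Enemy AI controller that runs the BT_EnemyAI behavior tree on possession and feeds it target and home data.
; On possess it also sets up BB_EnemyAI and stores the pawn's starting position as HomeLocation.
; A self-calling 0.2-second loop writes player character 0 to TargetActor without any sensing checks, and stops once that character is invalid.
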(event Custom|PerceiveEnvironmentLoop
  (bind _returnvalue (Game|GetPlayerCharacter 0))
  (Utilities|IsValid _returnvalue
    (:Is%20Valid
      (AI|Components|Blackboard|SetValueasObject (AI|GetBlackboard 0) (Utilities|Name|MakeLiteralName "TargetActor") _returnvalue)
      (Utilities|FlowControl|Delay 0.2)
      (CallFunction|PerceiveEnvironmentLoop))))

(event EventPossess
  (params (PossessedPawn :type Pawn%20Object%20Reference))
  (AI|RunBehaviorTree "/Game/Blueprints/EnemyAI/BT_EnemyAI.BT_EnemyAI")
  (CallFunction|PerceiveEnvironmentLoop)
  (bind _blackboardcomponent (Class|AIController|UseBlackboard "/Game/Blueprints/EnemyAI/BB_EnemyAI.BB_EnemyAI"))
  (AI|Components|Blackboard|SetValueasVector _blackboardcomponent (Utilities|Name|MakeLiteralName "HomeLocation") (Transformation|GetActorLocation PossessedPawn)))

(fn ConstructionScript)