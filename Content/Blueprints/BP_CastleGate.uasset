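; BP_CastleGate is the castle gate that serves as the win condition, gated on the player's collected flowers.
; When a BP_ThirdPersonCharacter overlaps GateTrigger, its FlowerCount is compared against RequiredFlowers.
; With enough flowers it shows WBP_WinScreen and switches player 0 to UI-only input with a visible cursor.
; Otherwise it only prints a message that more flowers are needed.
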(event OnComponentBeginOverlap(GateTrigger)
  (params (OverlappedComponent :type Primitive%20Component%20Object%20Reference) (OtherActor :type Actor%20Object%20Reference) (OtherComp :type Primitive%20Component%20Object%20Reference) (OtherBodyIndex :type Integer) (bFromSweep :type Boolean) (SweepResult :type Hit%20Result%20Structure%20%28by%20ref%29))
  (bind _returnvalue (Game|GetPlayerController 0))
  (bind _asbp_third_person_character (Utilities|Casting|CastToBP_ThirdPersonCharacter OtherActor))
  (if (>= (Variables|/Game/Blueprints/BP_ThirdPersonCharacter.BP_ThirdPersonCharacter_C|GetFlowerCount _asbp_third_person_character) (Variables|Default|GetRequiredFlowers))
    (bind _returnvalue_2 (UserInterface|CreateWidget "/Game/Blueprints/UI/WBP_WinScreen.WBP_WinScreen_C"))
    (UserInterface|Viewport|AddtoViewport _returnvalue_2 0)
    (Input|SetInputModeUIOnly _returnvalue 0 "DoNotLock" false)
    (Variables|/Script/Engine.PlayerController|SetbShowMouseCursor _returnvalue true)
    (else
      (Development|PrintString "NEED MORE FLOWERS"))))

(event EventBeginPlay)

(event Collision|EventActorBeginOverlap
  (params (OtherActor :type Actor%20Object%20Reference)))

(event EventTick
  (params (DeltaSeconds :type Float%20%28single-precision%29)))

(fn ConstructionScript)